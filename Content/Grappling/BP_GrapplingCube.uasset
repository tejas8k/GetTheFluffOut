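; BP_GrapplingCube is an actor that glides from an initial to a final location, with both seeded from its position at BeginPlay.
; Tick plays a timeline whenever the two locations differ and sets its time when they match.
; The timeline lerps the cube, sphere, billboard and widget components together in world space, then resets both locations to the actor's position on finish.
; This graph never sets a distinct destination itself.
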(event `self.ReceiveBeginPlay`
  (bind _returnvalue (`self.K2_GetActorLocation`))
  (set `self.InitialLocation` _returnvalue)
  (set `self.FinalLocation` _returnvalue))

(event `self.ReceiveTick`
  (params (DeltaSeconds :type "Float (single-precision)"))
  (bind _returnvalue (`self.K2_GetActorLocation`))
  (if (== (`self.InitialLocation`) (`self.FinalLocation`))
    (bind (_direction _newtrack_0) (`Timeline|Timeline_0` :!via `SetNewTime` :!label _label)
      (:`Update`
        (bind _returnvalue_2 (`KismetMathLibrary.VLerp` (`self.InitialLocation`) (`self.FinalLocation`) _newtrack_0))
        (`SceneComponent.K2_SetWorldLocation` (`self.Cube`) _returnvalue_2 false false)
        (`SceneComponent.K2_SetWorldLocation` (`self.Sphere`) _returnvalue_2 false false)
        (`SceneComponent.K2_SetWorldLocation` (`self.Billboard`) _returnvalue_2 false false)
        (`SceneComponent.K2_SetWorldLocation` (`self.Widget`) _returnvalue_2 false false))
      (:`Finished`
        (set `self.InitialLocation` _returnvalue)
        (set `self.FinalLocation` _returnvalue)))
    (else
      (goto _label))))

(fn `UserConstructionScript`
  (`parent.UserConstructionScript`))