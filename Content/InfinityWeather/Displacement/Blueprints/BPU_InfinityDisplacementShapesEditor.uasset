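; Editor utility actor for authoring Infinity Weather displacement shape lists against a previewed skeletal or static mesh.
; Construction and Draw feed the list through the displacement component into a stack, drawn as color-coded debug spheres, boxes, cylinders or capsules.
; Save writes the list to a data asset within a transaction, Load reads and redraws it, and Hide clears the drawing.
; The static-mesh branch also attaches shapes to SkeletalMesh.
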(fn `Draw`
  (locals (Stack :type "Array of /Game/InfinityWeather/Displacement/Blueprints/BS_DisplacementShape Structure") (ShapeTransform :type "Transform Structure"))
  (bind _shapetransform (`local.ShapeTransform`))
  (bind (_shapetransform_location _shapetransform_rotation _shapetransform_scale) (`KismetMathLibrary.BreakTransform` (`local.ShapeTransform`)))
  (bind _shapetransform_2 (`local.ShapeTransform`))
  (bind _shapetransform_3 (`local.ShapeTransform`))
  (bind _returnvalue (* (`KismetMathLibrary.GetUpVector` (.rotation _shapetransform)) (.z (.scale _shapetransform))))
  (`KismetSystemLibrary.FlushPersistentDebugLines` null)
  (set `/Game/InfinityWeather/Displacement/Blueprints/BP_InfinityDisplacementComponent.DisplacementShapesCustomList` (`self.List`) (`self.BP_InfinityDisplacementComponent`))
  (`/Game/InfinityWeather/Displacement/Blueprints/BP_InfinityDisplacementComponent.InitPreviousTransforms` (`self.BP_InfinityDisplacementComponent`))
  (`KismetArrayLibrary.Array_Clear` (`local.Stack`))
  (`|ExecutionSequence`
    (:`then_0`
      (`/Engine/EditorBlueprintResources/StandardMacros.IsValid` (`self.SkeletalMeshReference`)
        (:`Is Valid`
          (`/Game/InfinityWeather/Displacement/Blueprints/BP_InfinityDisplacementComponent.AttachDisplacementShapeData` (`self.BP_InfinityDisplacementComponent`) (`self.SkeletalMesh`) (`local.Stack`)))))
    (:`then_1`
      (`/Engine/EditorBlueprintResources/StandardMacros.IsValid` (`self.StaticMeshReference`)
        (:`Is Valid`
          (`/Game/InfinityWeather/Displacement/Blueprints/BP_InfinityDisplacementComponent.AttachDisplacementShapeData` (`self.BP_InfinityDisplacementComponent`) (`self.SkeletalMesh`) (`local.Stack`)))))
    (:`then_2`
      (for _array_element (`local.Stack`)
        (set `local.ShapeTransform` (`.Transform_46_B120AC2D41FD25FF4E14FF99E8D89E71` (break `/Game/InfinityWeather/Displacement/Blueprints/BS_DisplacementShape` _array_element)))
        (switch `/Game/InfinityWeather/Displacement/Blueprints/BE_DisplacementShape` (break `/Game/InfinityWeather/Displacement/Blueprints/BS_DisplacementShape` _array_element)
          (:`NewEnumerator0`
            (`KismetSystemLibrary.DrawDebugSphere` null (.location _shapetransform_2) (+ (.x (.scale _shapetransform_2)) 2.0) 12 (struct :`R` 0.494925 :`G` 0.274347 :`B` 1.0 :`A` 1.0) 100.0 0.5 :!label _label))
          (:`NewEnumerator6`
            (goto _label))
          (:`NewEnumerator1`
            (`KismetSystemLibrary.DrawDebugBox` null _shapetransform_location (* _shapetransform_scale 1.01) (struct :`R` 0.004275 :`G` 0.255208 :`B` 0.0512 :`A` 1.0) _shapetransform_rotation 100.0 0.5 :!label _label_2))
          (:`NewEnumerator9`
            (goto _label_2))
          (:`NewEnumerator4`
            (`KismetSystemLibrary.DrawDebugCylinder` null (+ (.location _shapetransform) _returnvalue) (- (.location _shapetransform) _returnvalue) (+ (.x (.scale _shapetransform)) 1.0) 16 (struct :`R` 0.588542 :`G` 0.431489 :`A` 1.0) 100.0 0.5))
          (:`NewEnumerator5`
            (`KismetSystemLibrary.DrawDebugCapsule` null (.location _shapetransform_3) (+ (.x (.scale _shapetransform_3)) (.z (.scale _shapetransform_3))) (+ (.x (.scale _shapetransform_3)) 2.0) (.rotation _shapetransform_3) (struct :`R` 1.0 :`B` 0.101973 :`A` 1.0) 100.0 0.5)))))))

(fn `Hide`
  (`KismetSystemLibrary.FlushPersistentDebugLines` null))

(fn `Load`
  (`/Engine/EditorBlueprintResources/StandardMacros.IsValid` (`self.Data`)
    (:`Is Valid`
      (set `self.List` (`/Game/InfinityWeather/Displacement/Blueprints/Presets/PDS_DisplacementShapes.Shapes` (`self.Data`)))
      (`self.Draw`))))

(fn `Save`
  (bind _data (`self.Data`))
  (`/Engine/EditorBlueprintResources/StandardMacros.IsValid` (`self.Data`)
    (:`Is Valid`
      (`KismetSystemLibrary.BeginTransaction` "" "" _data)
      (set `/Game/InfinityWeather/Displacement/Blueprints/Presets/PDS_DisplacementShapes.Shapes` (`self.List`) _data)
      (`KismetSystemLibrary.TransactObject` _data))))

(fn `UserConstructionScript`
  (`|ExecutionSequence`
    (:`then_0`
      (`/Engine/EditorBlueprintResources/StandardMacros.IsValid` (`self.SkeletalMeshReference`)
        (:`Is Valid`
          (`SkinnedMeshComponent.SetSkinnedAssetAndUpdate` (`self.SkeletalMesh`) (`self.SkeletalMeshReference`) true))))
    (:`then_1`
      (`/Engine/EditorBlueprintResources/StandardMacros.IsValid` (`self.StaticMeshReference`)
        (:`Is Valid`
          (`StaticMeshComponent.SetStaticMesh` (`self.StaticMesh`) (`self.StaticMeshReference`)))))
    (:`then_2`
      (`self.Draw`))))