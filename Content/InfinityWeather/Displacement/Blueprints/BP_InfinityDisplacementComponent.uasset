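; Actor component that supplies socket-attached displacement shapes for the Infinity Weather displacement system.
; It merges a custom list with an optional data asset, then appends each shape in world space to the supplied stack.
; Trail types cache previous transforms to bridge movement within a distance range: spheres stretch into capsules, wheels add a box behind their cylinder.
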(event `self.ReceiveBeginPlay`
  (`self.InitPreviousTransforms`))

(fn `AttachDisplacementShapeData`
  (params (Parent :type "SceneComponent Object Reference") (Stack :type "Array of /Game/InfinityWeather/Displacement/Blueprints/BS_DisplacementShape Structure (by ref)"))
  (locals (ShapeData :type "/Game/InfinityWeather/Displacement/Blueprints/BS_DisplacementSocketShape Structure") (OldTransform :type "Transform Structure") (NewTransform :type "Transform Structure") (MoveDistance :type "Float (double-precision)" :default 0.0))
  (bind (_tracelengthminmax_x _tracelengthminmax_y) (`KismetMathLibrary.BreakVector2D` (`self.TraceLengthMinMax`)))
  (bind _oldtransform_location (`KismetMathLibrary.BreakTransform` (`local.OldTransform`)))
  (bind _oldtransform_location_2 (`KismetMathLibrary.BreakTransform` (`local.OldTransform`)))
  (bind _newtransform_location (`KismetMathLibrary.BreakTransform` (`local.NewTransform`)))
  (bind (_newtransform_location_2 _newtransform_rotation) (`KismetMathLibrary.BreakTransform` (`local.NewTransform`)))
  (bind _newtransform (`local.NewTransform`))
  (bind _shapedata (`local.ShapeData`))
  (bind _oldtransform_location_3 (`KismetMathLibrary.BreakTransform` (`local.OldTransform`)))
  (bind _newtransform_location_3 (`KismetMathLibrary.BreakTransform` (`local.NewTransform`)))
  (bind _oldtransform_location_4 (`KismetMathLibrary.BreakTransform` (`local.OldTransform`)))
  (bind _newtransform_location_4 (`KismetMathLibrary.BreakTransform` (`local.NewTransform`)))
  (bind _newtransform_2 (`local.NewTransform`))
  (bind (_tracelengthminmax_x_2 _tracelengthminmax_y_2) (`KismetMathLibrary.BreakVector2D` (`self.TraceLengthMinMax`)))
  (bind _shapedata_2 (`local.ShapeData`))
  (bind _shapedata_3 (`local.ShapeData`))
  (`/Engine/EditorBlueprintResources/StandardMacros.IsValid` Parent
    (:`Is Valid`
      (for (_array_element _array_index) (`self.CombinedShapes`)
        (set `local.ShapeData` _array_element)
        (switch `/Game/InfinityWeather/Displacement/Blueprints/BE_DisplacementShape` (break `/Game/InfinityWeather/Displacement/Blueprints/BS_DisplacementShape` (`.Shape_24_583F12CD45C42ACE5BAEB78E558AE074` (break `/Game/InfinityWeather/Displacement/Blueprints/BS_DisplacementSocketShape` (`local.ShapeData`))))
          (:`NewEnumerator0`
            ;[1 1 1] Attached to component
            (`KismetArrayLibrary.Array_Add` (`local.Stack`) (make `/Game/InfinityWeather/Displacement/Blueprints/BS_DisplacementShape` (break `/Game/InfinityWeather/Displacement/Blueprints/BS_DisplacementShape` (`.Shape_24_583F12CD45C42ACE5BAEB78E558AE074` (break `/Game/InfinityWeather/Displacement/Blueprints/BS_DisplacementSocketShape` _shapedata_2))) (`.Intensity_65_6AD371EC45C33B6868E3A38617FCB979` (break `/Game/InfinityWeather/Displacement/Blueprints/BS_DisplacementShape` (`.Shape_24_583F12CD45C42ACE5BAEB78E558AE074` (break `/Game/InfinityWeather/Displacement/Blueprints/BS_DisplacementSocketShape` _shapedata_2)))) (`KismetMathLibrary.ComposeTransforms` (`.Transform_46_B120AC2D41FD25FF4E14FF99E8D89E71` (break `/Game/InfinityWeather/Displacement/Blueprints/BS_DisplacementShape` (`.Shape_24_583F12CD45C42ACE5BAEB78E558AE074` (break `/Game/InfinityWeather/Displacement/Blueprints/BS_DisplacementSocketShape` _shapedata_2)))) (`SceneComponent.GetSocketTransform` (`local.Parent`) (break `/Game/InfinityWeather/Displacement/Blueprints/BS_DisplacementSocketShape` _shapedata_2) "RTS_World")) (`.Pattern_64_E169050C4EF699A1F28D369B40805FDD` (break `/Game/InfinityWeather/Displacement/Blueprints/BS_DisplacementShape` (`.Shape_24_583F12CD45C42ACE5BAEB78E558AE074` (break `/Game/InfinityWeather/Displacement/Blueprints/BS_DisplacementSocketShape` _shapedata_2))))) :!label _label))
          (:`NewEnumerator6`
            (goto _label))
          (:`NewEnumerator1`
            (goto _label))
          (:`NewEnumerator9`
            (goto _label))
          (:`NewEnumerator4`
            (goto _label))
          (:`NewEnumerator5`
            (goto _label))
          (:`NewEnumerator10`
            (goto _label))
          (:`NewEnumerator12`
            (goto _label))
          (:`NewEnumerator11`
            (goto _label))
          (:`NewEnumerator13`
            (goto _label))
          (:`NewEnumerator15`
            (goto _label))
          (:`NewEnumerator16`
            (set `local.OldTransform` (`|GetArrayItem` (`self.PreviousTransforms`) _array_index) :!label _label_2)
            (set `local.NewTransform` (`KismetMathLibrary.ComposeTransforms` (`.Transform_46_B120AC2D41FD25FF4E14FF99E8D89E71` (break `/Game/InfinityWeather/Displacement/Blueprints/BS_DisplacementShape` (`.Shape_24_583F12CD45C42ACE5BAEB78E558AE074` (break `/Game/InfinityWeather/Displacement/Blueprints/BS_DisplacementSocketShape` _shapedata_3)))) (`SceneComponent.GetSocketTransform` (`local.Parent`) (break `/Game/InfinityWeather/Displacement/Blueprints/BS_DisplacementSocketShape` _shapedata_3) "RTS_World")))
            (`KismetArrayLibrary.Array_Set` (`self.PreviousTransforms`) _array_index (`local.NewTransform`) true)
            (switch `/Game/InfinityWeather/Displacement/Blueprints/BE_DisplacementShape` (break `/Game/InfinityWeather/Displacement/Blueprints/BS_DisplacementShape` (`.Shape_24_583F12CD45C42ACE5BAEB78E558AE074` (break `/Game/InfinityWeather/Displacement/Blueprints/BS_DisplacementSocketShape` (`local.ShapeData`))))
              (:`NewEnumerator16`
                ;[1 1 1] Sphere trace
                (if (== (`local.OldTransform`) (`KismetMathLibrary.MakeTransform` (0.0 0.0 0.0)))
                  (`KismetArrayLibrary.Array_Add` (`local.Stack`) (make `/Game/InfinityWeather/Displacement/Blueprints/BS_DisplacementShape` "NewEnumerator0" (`.Intensity_65_6AD371EC45C33B6868E3A38617FCB979` (break `/Game/InfinityWeather/Displacement/Blueprints/BS_DisplacementShape` (`.Shape_24_583F12CD45C42ACE5BAEB78E558AE074` (break `/Game/InfinityWeather/Displacement/Blueprints/BS_DisplacementSocketShape` _shapedata)))) (`local.NewTransform`)) :!label _label_3)
                  (else
                    (bind _output_get (set `local.MoveDistance` (`KismetMathLibrary.Vector_Distance` _oldtransform_location_3 _newtransform_location_3)))
                    (if (`KismetMathLibrary.InRange_FloatFloat` _output_get _tracelengthminmax_x_2 _tracelengthminmax_y_2)
                      (`KismetArrayLibrary.Array_Add` (`local.Stack`) (make `/Game/InfinityWeather/Displacement/Blueprints/BS_DisplacementShape` "NewEnumerator5" (`.Intensity_65_6AD371EC45C33B6868E3A38617FCB979` (break `/Game/InfinityWeather/Displacement/Blueprints/BS_DisplacementShape` (`.Shape_24_583F12CD45C42ACE5BAEB78E558AE074` (break `/Game/InfinityWeather/Displacement/Blueprints/BS_DisplacementSocketShape` _shapedata)))) (`KismetMathLibrary.MakeTransform` (`KismetMathLibrary.VLerp` _oldtransform_location_4 _newtransform_location_4 0.5) (`KismetMathLibrary.MakeRotFromZ` (- _oldtransform_location_4 _newtransform_location_4)) (`KismetMathLibrary.MakeVector` (.x (.scale _newtransform_2)) (.x (.scale _newtransform_2)) (* (`local.MoveDistance`) 0.5)))))
                      (else
                        (goto _label_3))))))
              (:`NewEnumerator17`
                ;[1 1 1] Box trace
                (`|ExecutionSequence`
                  (:`then_0`
                    (`KismetArrayLibrary.Array_Add` (`local.Stack`) (make `/Game/InfinityWeather/Displacement/Blueprints/BS_DisplacementShape` "NewEnumerator4" (`.Intensity_65_6AD371EC45C33B6868E3A38617FCB979` (break `/Game/InfinityWeather/Displacement/Blueprints/BS_DisplacementShape` (`.Shape_24_583F12CD45C42ACE5BAEB78E558AE074` (break `/Game/InfinityWeather/Displacement/Blueprints/BS_DisplacementSocketShape` (`local.ShapeData`))))) (`local.NewTransform`))))
                  (:`then_1`
                    (if (not (== (`local.OldTransform`) (`KismetMathLibrary.MakeTransform` (0.0 0.0 0.0))))
                      (bind _output_get_2 (set `local.MoveDistance` (`KismetMathLibrary.Vector_Distance` _oldtransform_location_2 _newtransform_location)))
                      (if (`KismetMathLibrary.InRange_FloatFloat` _output_get_2 _tracelengthminmax_x _tracelengthminmax_y)
                        (`KismetArrayLibrary.Array_Add` (`local.Stack`) (make `/Game/InfinityWeather/Displacement/Blueprints/BS_DisplacementShape` "NewEnumerator1" (`.Intensity_65_6AD371EC45C33B6868E3A38617FCB979` (break `/Game/InfinityWeather/Displacement/Blueprints/BS_DisplacementShape` (`.Shape_24_583F12CD45C42ACE5BAEB78E558AE074` (break `/Game/InfinityWeather/Displacement/Blueprints/BS_DisplacementSocketShape` (`local.ShapeData`))))) (`KismetMathLibrary.MakeTransform` (`KismetMathLibrary.VLerp` _oldtransform_location _newtransform_location_2 0.5) (`KismetMathLibrary.MakeRotFromXZ` (`KismetMathLibrary.GetUpVector` _newtransform_rotation) (- _oldtransform_location _newtransform_location_2)) (`KismetMathLibrary.MakeVector` (.z (.scale _newtransform)) (.x (.scale _newtransform)) (* (`local.MoveDistance`) 0.5))))))))))))
          (:`NewEnumerator17`
            (goto _label_2)))))))

(fn `InitPreviousTransforms`
  (set `self.CombinedShapes` (`self.DisplacementShapesCustomList`))
  (`/Engine/EditorBlueprintResources/StandardMacros.IsValid` (`self.DisplacementShapesDataAsset`)
    (:`Is Valid`
      (`KismetArrayLibrary.Array_Append` (`self.CombinedShapes`) (`/Game/InfinityWeather/Displacement/Blueprints/Presets/PDS_DisplacementShapes.Shapes` (`self.DisplacementShapesDataAsset`))))
    (:`Is Not Valid`
      _))
  (set `self.PreviousTransforms` (`|MakeArray`))
  (`KismetArrayLibrary.Array_Resize` (`self.PreviousTransforms`) (`KismetArrayLibrary.Array_Length` (`self.CombinedShapes`))))

(fn `SetCombinedShapes`
  (params (CombinedShapes :type "Array of /Game/InfinityWeather/Displacement/Blueprints/BS_DisplacementSocketShape Structure"))
  (set `self.CombinedShapes` CombinedShapes))

(fn `SetDisplacementShapesDataAsset`
  (params (ShapesDataAsset :type "/Game/InfinityWeather/Displacement/Blueprints/Presets/PDS_DisplacementShapes Object Reference"))
  (set `self.DisplacementShapesDataAsset` ShapesDataAsset)
  (`self.InitPreviousTransforms`))