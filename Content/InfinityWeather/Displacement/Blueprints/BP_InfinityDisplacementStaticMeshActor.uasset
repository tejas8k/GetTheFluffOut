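; Static mesh actor that supplies a displacement shape to the Infinity Weather displacement system.
; SaveSelf caches the shape data on construction and BeginPlay, and flags the actor as dynamic if its mesh component is Movable.
; When asked to add its shape to a stack, dynamic actors refresh the transform through GetShapeTransform, while non-movable ones add the cached data unchanged.
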(event `self.ReceiveBeginPlay`
  (`self.SaveSelf`))

(fn `AddDisplacementShapeData`
  (params (Stack :type "Array of /Game/InfinityWeather/Displacement/Blueprints/BS_DisplacementShape Structure (by ref)"))
  (returns (Added :type Boolean))
  (if (`self.IsDynamic`)
    (bind _structout (setmembers `/Game/InfinityWeather/Displacement/Blueprints/BS_DisplacementShape` :`StructRef` (`self.StaticShapeData`) :`Transform` (`self.GetShapeTransform`)))
    (`KismetArrayLibrary.Array_Add` Stack _structout)
    (return true)
    (else
      (`KismetArrayLibrary.Array_Add` Stack (`self.StaticShapeData`))
      (return true))))

(fn `SaveSelf`
  (bind (_shapedata_type _shapedata_intensity _shapedata_transform _shapedata_pattern) (break `/Game/InfinityWeather/Displacement/Blueprints/BS_DisplacementShape` (`self.ShapeData`)))
  (set `self.StaticShapeData` (make `/Game/InfinityWeather/Displacement/Blueprints/BS_DisplacementShape` _shapedata_type _shapedata_intensity "0.000000,0.000000,0.000000|0.000000,0.000000,0.000000|50.000000,50.000000,50.000000" _shapedata_pattern))
  (set `self.IsDynamic` (`|EnumEquality` (`SceneComponent.Mobility` (`self.StaticMeshComponent`)) "Movable")))

(fn `UserConstructionScript`
  (`self.SaveSelf`))