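; Displacement decal actor in InfinityWeather that supplies a textured shape to a displacement stack.
; AddDisplacementShapeData appends its type, intensity, pattern and transform, composed with the actor transform on each call; a static-data caching branch is left unconnected.
; Construction shows the pattern on a preview mesh through a dynamic material, with visibility set by EditorPreview.
; BeginPlay hides the Box and, given a positive LifeTime, destroys the actor after that delay.
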(event `self.ReceiveBeginPlay`
  (bind _box (`self.Box`))
  (`parent.ReceiveBeginPlay`)
  (`/Engine/EditorBlueprintResources/StandardMacros.IsValid` _box
    (:`Is Valid`
      (`SceneComponent.SetVisibility` _box false false)
      (if (> (`self.LifeTime`) 0.0)
        (`KismetSystemLibrary.Delay` (`self.LifeTime`))
        (`self.K2_DestroyActor`)))))

(fn `AddDisplacementShapeData`
  (params (Stack :type "Array of /Game/InfinityWeather/Displacement/Blueprints/BS_DisplacementShape Structure (by ref)"))
  (returns (Added :type Boolean))
  (bind (_shapedata_type _shapedata_intensity _shapedata_transform _shapedata_pattern) (break `/Game/InfinityWeather/Displacement/Blueprints/BS_DisplacementShape` (`self.ShapeData`)))
  (`KismetArrayLibrary.Array_Add` (`local.Stack`) (make `/Game/InfinityWeather/Displacement/Blueprints/BS_DisplacementShape` _shapedata_type _shapedata_intensity (`KismetMathLibrary.ComposeTransforms` _shapedata_transform (`self.GetTransform`)) _shapedata_pattern))
  (return true))

(fn `UserConstructionScript`
  (bind (_shapedata_type _shapedata_intensity _shapedata_transform _shapedata_pattern) (break `/Game/InfinityWeather/Displacement/Blueprints/BS_DisplacementShape` (`self.ShapeData`)))
  (`parent.UserConstructionScript`)
  (bind _returnvalue (`PrimitiveComponent.CreateDynamicMaterialInstance` (`self.StaticMeshComponent`) 0 "/Game/InfinityWeather/Displacement/Capture/M_DecalPreview.M_DecalPreview" "None"))
  (`MaterialInstanceDynamic.SetTextureParameterValue` _returnvalue "Texture" _shapedata_pattern)
  (`SceneComponent.SetVisibility` (`self.StaticMeshComponent`) (`self.EditorPreview`) false))