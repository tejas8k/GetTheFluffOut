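; Footstep component that spawns surface-dependent particle and audio effects at bone sockets, as one-shots or movement-driven loops.
; BeginPlay instantiates preset templates into a map keyed by a combined surface and modifier integer.
; A downward sphere trace picks the preset from physical material, overridden by the highest-priority active volume.
; Tick swaps or stops loop effects as bones move, while tracked one-shot emitters follow custom time dilation.
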(event `self.ReceiveBeginPlay`
  (`self.Initialize`))

(event `self.ReceiveTick`
  (params (DeltaSeconds :type "Float (single-precision)"))
  (`self.UpdateLoops`))

(fn `ActivateLoops`
  (params (Mesh :type "SkeletalMeshComponent Object Reference"))
  (bind _values (`BlueprintMapLibrary.Map_Values` (`self.AttachementLoops`)))
  (for _array_element _values
    (`self.Loop` _array_element Mesh))
  (`self.UpdateLoops`))

(fn `FindFootstepPreset`
  (params (Mesh :type "PrimitiveComponent Object Reference") (Attachement :type "/Game/InfinityWeather/Footstep/Blueprints/BS_FootstepAttachement Structure"))
  (returns (Preset :type "/Game/InfinityWeather/Footstep/Presets/BP_FootstepPreset Object Reference"))
  (locals (LFootstepInstance :type "/Game/InfinityWeather/Footstep/Presets/BP_FootstepPreset Object Reference") (SocketLocation :type "Vector Structure" :default (0.0 0.0 0.0)) (SurfaceType :type "EPhysicalSurface Enum" :default "SurfaceType_Default"))
  (bind (_attachement_bone _attachement_transform _attachement_modifier) (break `/Game/InfinityWeather/Footstep/Blueprints/BS_FootstepAttachement` (`local.Attachement`)))
  ;[1 0.576 0.6258] Trace ground test
  (if (`self.IsActive`)
    (set `local.SocketLocation` (`SceneComponent.GetSocketLocation` (`local.Mesh`) (`.Bone_2_8C52E8664CD1E2061AC7CB856D1FDA3F` (break `/Game/InfinityWeather/Footstep/Blueprints/BS_FootstepAttachement` (`local.Attachement`)))))
    (bind (_outhit _returnvalue) (`KismetSystemLibrary.SphereTraceSingleForObjects` (+ (`local.SocketLocation`) (`KismetMathLibrary.MakeVector` 0.0 0.0 (`self.FootSize`))) (- (`local.SocketLocation`) (`KismetMathLibrary.MakeVector` 0.0 0.0 (`self.TraceDepth`))) 10.0 (`|MakeArray` "ObjectTypeQuery1" :!type "EObjectTypeQuery Enum") false (`|MakeArray` (`self.GetOwner` (`local.Mesh`))) "None" true (struct :`R` 1.0 :`A` 1.0) (struct :`G` 1.0 :`A` 1.0) 1.0))
    (if _returnvalue
      ;[0.8415 1 0.6431] Preset identification based on surface type
      (`|ExecutionSequence`
        (:`then_0`
          (bind _volume (`self.GetOverrideVolume`))
          (`/Engine/EditorBlueprintResources/StandardMacros.IsValid` _volume
            (:`Is Valid`
              (set `local.SurfaceType` (`/Game/InfinityWeather/Footstep/Blueprints/BP_FootstepVolume.SurfaceType` _volume)))
            (:`Is Not Valid`
              (bind (_bblockinghit _binitialoverlap _time _distance _location _impactpoint _normal _impactnormal _physmat) (`GameplayStatics.BreakHitResult` _outhit))
              (`/Engine/EditorBlueprintResources/StandardMacros.IsValid` _physmat
                (:`Is Valid`
                  (set `local.SurfaceType` (`PhysicalMaterial.SurfaceType` _physmat)))
                (:`Is Not Valid`
                  (set `local.SurfaceType` (`local.SurfaceType`))))))
          (set `local.LFootstepInstance` (`BlueprintMapLibrary.Map_Find` (`self.Instances`) (`self.MapFootstep` (`local.SurfaceType`) _attachement_modifier))))
        (:`then_1`
          (return (`local.LFootstepInstance`))))
      (else
        (set `local.LFootstepInstance` null)))))

(fn `GetOverrideVolume`
  (returns (Volume :type "/Game/InfinityWeather/Footstep/Blueprints/BP_FootstepVolume Object Reference"))
  (locals (CurrentVolume :type "/Game/InfinityWeather/Footstep/Blueprints/BP_FootstepVolume Object Reference") (Temp :type "/Game/InfinityWeather/Footstep/Blueprints/BP_FootstepVolume Object Reference"))
  (bind _returnvalue (`KismetArrayLibrary.Array_LastIndex` (`self.OverrideVolumes`)))
  ;[1 1 1] Looking for volume lasy is most important (priority)
  (set `local.CurrentVolume` null)
  (`|ExecutionSequence`
    (:`then_0`
      (for _index (range (+ _returnvalue 1))
        (set `local.Temp` (`|GetArrayItem` (`self.OverrideVolumes`) (- _returnvalue _index)))
        (if (`/Game/InfinityWeather/Footstep/Blueprints/BP_FootstepVolume.IsActive` (`local.Temp`))
          (set `local.CurrentVolume` (`local.Temp`))
          (break))))
    (:`then_1`
      (return (`local.CurrentVolume`)))))

(fn `Initialize`
  (locals (OwnerAttachComponents :type "Array of ActorComponent Object Reference"))
  (`|ExecutionSequence`
    (:`then_0`
      (`BlueprintMapLibrary.Map_Clear` (`self.Instances`))
      (bind _keys (`BlueprintMapLibrary.Map_Keys` (`self.Templates`)))
      (for _array_element _keys
        (bind _value (`BlueprintMapLibrary.Map_Find` (`self.Templates`) _array_element))
        (bind _keys_2 (`BlueprintMapLibrary.Map_Keys` (break `/Game/InfinityWeather/Footstep/Blueprints/BS_FootstepTemplate` _value)))
        (for _array_element_2 _keys_2
          (bind _returnvalue (`|GenericCreateObject` (`BlueprintMapLibrary.Map_Find` (break `/Game/InfinityWeather/Footstep/Blueprints/BS_FootstepTemplate` _value) _array_element_2) self))
          (`BlueprintMapLibrary.Map_Add` (`self.Instances`) (`self.MapFootstep` _array_element_2 _array_element) _returnvalue))))))

(fn `Loop`
  (params (Attachement :type "/Game/InfinityWeather/Footstep/Blueprints/BS_FootstepAttachement Structure") (Mesh :type "SkeletalMeshComponent Object Reference") (VelocityMin :type "Float (double-precision)"))
  (`KismetArrayLibrary.Array_Add` (`self.ActiveLoops`) (make `/Game/InfinityWeather/Footstep/Blueprints/BS_FootstepLoop` true Mesh Attachement)))

(fn `MapFootstep`
  (params (Surface :type "EPhysicalSurface Enum" :default "SurfaceType_Default") (Modififer :type "/Game/InfinityWeather/Footstep/Blueprints/BE_FootstepModifier Enum" :default "NewEnumerator2"))
  (returns (Index :type Integer))
  (return (`KismetMathLibrary.Conv_ByteToInt` (+ Surface (* Modififer 100)))))

(fn `Play`
  (params (Attachement :type "/Game/InfinityWeather/Footstep/Blueprints/BS_FootstepAttachement Structure") (Intensity :type "Float (double-precision)") (Mesh :type "SkeletalMeshComponent Object Reference"))
  (locals (LFootstepInstance :type "/Game/InfinityWeather/Footstep/Presets/BP_FootstepPreset Object Reference"))
  (if (`self.IsActive`)
    (bind _preset (`self.FindFootstepPreset` Mesh Attachement))
    (set `local.LFootstepInstance` _preset)
    ;[1 0.6384 0.4536] Final play effect
    (`/Engine/EditorBlueprintResources/StandardMacros.IsValid` (`local.LFootstepInstance`)
      (:`Is Valid`
        (bind _spawnedemitter (`/Game/InfinityWeather/Footstep/Presets/BP_FootstepPreset.Spawn` (`local.LFootstepInstance`) (`local.Mesh`) (`local.Attachement`) (`local.Intensity`)))
        (`/Engine/EditorBlueprintResources/StandardMacros.IsValid` _spawnedemitter
          (:`Is Valid`
            (if (not (== (`self.Dilation`) 1.0))
              (set `ParticleSystemComponent.CustomTimeDilation` (`self.Dilation`) _spawnedemitter))
            (bind _returnvalue (`KismetArrayLibrary.Array_Add` (`self.Emitters`) (`|ConvertAsset` _spawnedemitter)))
            (if (> _returnvalue (`self.MaxEmitters`))
              (`self.UpdateEmitters`))))))))

(fn `RemoveLoopEffects`
  (params (Attachemtn :type "/Game/InfinityWeather/Footstep/Blueprints/BS_FootstepLoop Structure (by ref)"))
  (bind (_active _parent _attachement _preset _particle _audio) (break `/Game/InfinityWeather/Footstep/Blueprints/BS_FootstepLoop` Attachemtn))
  (`/Engine/EditorBlueprintResources/StandardMacros.IsValid` _particle
    (:`Is Valid`
      (`self.Deactivate` _particle)
      (`/Engine/EditorBlueprintResources/StandardMacros.IsValid` _audio
        (:`Is Valid`
          (`self.Deactivate` _audio))))))

(fn `SetCustomDilation`
  (params (Dilation :type "Float (double-precision)"))
  (set `self.Dilation` Dilation)
  (bind (_arrayindex _arrayelement) (`/Engine/EditorBlueprintResources/StandardMacros.ReverseForEachLoop` (`self.Emitters`))
    (:`LoopBody`
      (if (`KismetSystemLibrary.IsValidSoftObjectReference` _arrayelement)
        (bind _output (`|ConvertAsset` _arrayelement))
        (`/Engine/EditorBlueprintResources/StandardMacros.IsValid` _output
          (:`Is Valid`
            (if (`self.IsBeingDestroyed` _output)
              (`KismetArrayLibrary.Array_Remove` (`self.Emitters`) _arrayindex :!label _label)
              (else
                (set `ParticleSystemComponent.CustomTimeDilation` (`self.Dilation`) _output))))
          (:`Is Not Valid`
            (goto _label)))
        (else
          (goto _label))))))

(fn `SetOverrideVolume`
  (params (Volume :type "/Game/InfinityWeather/Footstep/Blueprints/BP_FootstepVolume Object Reference") (Active :type Boolean))
  (locals (InsertPosition :type Integer))
  (if Active
    (if (not (>= (`KismetArrayLibrary.Array_Find` (`self.OverrideVolumes`) (`local.Volume`)) 0))
      (set `local.InsertPosition` (`KismetArrayLibrary.Array_Length` (`self.OverrideVolumes`)))
      (for (_array_element _array_index) (`self.OverrideVolumes`)
        (if (< (`/Game/InfinityWeather/Footstep/Blueprints/BP_FootstepVolume.Priority` (`local.Volume`)) (`/Game/InfinityWeather/Footstep/Blueprints/BP_FootstepVolume.Priority` _array_element))
          (set `local.InsertPosition` _array_index)
          (break)))
      (`KismetArrayLibrary.Array_Insert` (`self.OverrideVolumes`) (`local.Volume`) (`local.InsertPosition`)))
    (else
      (`KismetArrayLibrary.Array_RemoveItem` (`self.OverrideVolumes`) (`local.Volume`)))))

(fn `UpdateEmitters`
  (bind (_arrayindex _arrayelement) (`/Engine/EditorBlueprintResources/StandardMacros.ReverseForEachLoop` (`self.Emitters`))
    (:`LoopBody`
      (if (`KismetSystemLibrary.IsValidSoftObjectReference` _arrayelement)
        (bind _output (`|ConvertAsset` _arrayelement))
        (`/Engine/EditorBlueprintResources/StandardMacros.IsValid` _output
          (:`Is Valid`
            (if (`self.IsBeingDestroyed` _output)
              (`KismetArrayLibrary.Array_Remove` (`self.Emitters`) _arrayindex :!label _label)))
          (:`Is Not Valid`
            (goto _label)))
        (else
          (goto _label))))))

(fn `UpdateLoops`
  (locals (Element :type "/Game/InfinityWeather/Footstep/Blueprints/BS_FootstepLoop Structure") (NewPreset :type "/Game/InfinityWeather/Footstep/Presets/BP_FootstepPreset Object Reference") (ElementID :type Integer) (NewLocation :type "Vector Structure"))
  (bind (_element_active _element_parent _element_attachement) (break `/Game/InfinityWeather/Footstep/Blueprints/BS_FootstepLoop` (`local.Element`)))
  (bind (_element_active_2 _element_parent_2 _element_attachement_2) (break `/Game/InfinityWeather/Footstep/Blueprints/BS_FootstepLoop` (`local.Element`)))
  (bind (_element_active_3 _element_parent_3 _element_attachement_3 _element_preset) (break `/Game/InfinityWeather/Footstep/Blueprints/BS_FootstepLoop` (`local.Element`)))
  (bind (_element_active_4 _element_parent_4 _element_attachement_4 _element_preset_2) (break `/Game/InfinityWeather/Footstep/Blueprints/BS_FootstepLoop` (`local.Element`)))
  (bind (_element_active_5 _element_parent_5 _element_attachement_5 _element_preset_3) (break `/Game/InfinityWeather/Footstep/Blueprints/BS_FootstepLoop` (`local.Element`)))
  (bind ((`Parent_29_3B2DE5CC4236E0ADAB30E4BED5E4166D` _parent) (`Attachement_26_8C52E8664CD1E2061AC7CB856D1FDA3F` _attachement)) (break `/Game/InfinityWeather/Footstep/Blueprints/BS_FootstepLoop` (`local.Element`)))
  (for (_array_element _array_index) (`self.ActiveLoops`)
    (set `local.Element` _array_element)
    (set `local.ElementID` _array_index)
    (if _element_active_2
      (bind _output_get (set `local.NewLocation` (`SceneComponent.GetSocketLocation` _element_parent_2 (`.Bone_2_8C52E8664CD1E2061AC7CB856D1FDA3F` (break `/Game/InfinityWeather/Footstep/Blueprints/BS_FootstepAttachement` _element_attachement_2)))))
      (if (> (`KismetMathLibrary.VSize` (- _output_get (`.PreviousLocation_37_D9FEE9F4422548814CF8FA80A4BBA1C2` (break `/Game/InfinityWeather/Footstep/Blueprints/BS_FootstepLoop` (`local.Element`))))) (`self.MinVelovity`))
        (bind _preset (`self.FindFootstepPreset` _parent _attachement))
        (set `local.NewPreset` _preset)
        (else
          (set `local.NewPreset` null)))
      (setmembers `/Game/InfinityWeather/Footstep/Blueprints/BS_FootstepLoop` :`StructRef` (`|GetArrayItem` (`self.ActiveLoops`) (`local.ElementID`)) :`PreviousLocation` (`local.NewLocation`))
      (`/Engine/EditorBlueprintResources/StandardMacros.IsValid` (`local.NewPreset`)
        (:`Is Valid`
          (if (== _element_preset_2 (`local.NewPreset`))
            _
            (elif (== _element_preset null)
              (bind (_spawnedemitter _spawnedaudio) (`/Game/InfinityWeather/Footstep/Presets/BP_FootstepPreset.Spawn` (`local.NewPreset`) _element_parent _element_attachement 1.0 :!label _label))
              (setmembers `/Game/InfinityWeather/Footstep/Blueprints/BS_FootstepLoop` :`StructRef` (`|GetArrayItem` (`self.ActiveLoops`) (`local.ElementID`)) :`Preset` (`local.NewPreset`) :`Particle` _spawnedemitter :`Audio` _spawnedaudio)
              (else
                (`|ExecutionSequence`
                  (:`then_0`
                    (`self.RemoveLoopEffects` (`local.Element`)))
                  (:`then_1`
                    (goto _label)))))))
        (:`Is Not Valid`
          (if (not (== _element_preset_3 null))
            (`self.RemoveLoopEffects` (`local.Element`))
            (setmembers `/Game/InfinityWeather/Footstep/Blueprints/BS_FootstepLoop` :`StructRef` (`|GetArrayItem` (`self.ActiveLoops`) (`local.ElementID`)) :`Preset` null :`Particle` null :`Audio` null)))))))