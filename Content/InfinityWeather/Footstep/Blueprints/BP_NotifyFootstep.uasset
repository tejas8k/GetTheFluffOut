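; BP_NotifyFootstep is an animation notify that triggers InfinityWeather footsteps on the animated mesh's owner.
; It finds the owner's BP_InfinityFootstepComponent and resolves the selected attachment from its Attachements map, keeping the notify's custom attachment for one enum option when a bone is set.
; It then calls Play on the component with the attachment, intensity and mesh.
; The notify's displayed name derives from the attachment enum.
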(fn `GetNotifyName`
  (returns (ReturnValue :type String))
  (return (`KismetStringLibrary.Concat_StrStr` "FootStep_" (`|GetEnumeratorNameAsString` (`self.Attachement`)))))

(fn `Received_Notify`
  (params (MeshComp :type "SkeletalMeshComponent Object Reference") (Animation :type "AnimSequenceBase Object Reference"))
  (returns (ReturnValue :type Boolean))
  (locals (LComponent :type "/Game/InfinityWeather/Footstep/Blueprints/BP_InfinityFootstepComponent Object Reference") (LAttachement :type "/Game/InfinityWeather/Footstep/Blueprints/BS_FootstepAttachement Structure"))
  (bind _lattachement_bone (break `/Game/InfinityWeather/Footstep/Blueprints/BS_FootstepAttachement` (`local.LAttachement`)))
  (bind (_value _returnvalue) (`BlueprintMapLibrary.Map_Find` (`/Game/InfinityWeather/Footstep/Blueprints/BP_InfinityFootstepComponent.Attachements` (`local.LComponent`)) (`self.Attachement`)))
  (set `local.LComponent` (`Actor.GetComponentByClass` (`ActorComponent.GetOwner` MeshComp) "/Game/InfinityWeather/Footstep/Blueprints/BP_InfinityFootstepComponent.BP_InfinityFootstepComponent_C"))
  (`/Engine/EditorBlueprintResources/StandardMacros.IsValid` (`local.LComponent`)
    (:`Is Valid`
      (set `local.LAttachement` (`self.CustomAttachement`))
      (`|ExecutionSequence`
        (:`then_0`
          ;[1 1 1] Finding bone name
          (if (`|EnumEquality` (`self.Attachement`) "NewEnumerator2")
            (if (== "None" _lattachement_bone)
              (if _returnvalue :!label _label
                (set `local.LAttachement` _value)))
            (else
              (goto _label))))
        (:`then_1`
          (`/Game/InfinityWeather/Footstep/Blueprints/BP_InfinityFootstepComponent.Play` (`local.LComponent`) (`local.LAttachement`) (`self.Intensity`) (`local.MeshComp`))
          (return false))))))