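; Base precipitation actor for Infinity Weather that renders camera-box particles within a box volume or unbounded, with attenuated audio, and registers with the weather controller.
; A dynamic material receives forces from gravity, wind and randomness, crossfading old and new values as wind direction blends.
; Particle count blends over time, drives audio fade and selects power-of-two meshes, optionally async-loaded.
; A point query reports rain, snow, wind and force.
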(event `self.ReceiveBeginPlay`
  ;[1 1 1] Initialize precipitation effect
  (`/Engine/EditorBlueprintResources/StandardMacros.IsValid` (`self.Controller`)
    (:`Is Valid`
      (`self.SetController` (`self.Controller`)))
    (:`Is Not Valid`
      (bind _returnvalue (`GameplayStatics.GetActorOfClass` "/Game/InfinityWeather/Weather/Blueprints/BP_InfinityWeatherController.BP_InfinityWeatherController_C"))
      (`self.SetController` _returnvalue))))

(event `AsyncLoadMesh`
  (params (MeshRef :type "Object Soft Object Reference"))
  (if (`self.UseAsyncLoading`)
    (bind _object (`|LoadAsset` MeshRef)
      (:`Completed`
        (bind _asstatic_mesh (cast `StaticMesh` _object))
        (bind _output_get (set `self.UseStaticMesh` _asstatic_mesh))))
    (else
      (bind _returnvalue (`KismetSystemLibrary.LoadAsset_Blocking` MeshRef))
      (bind _asstatic_mesh_2 (cast `StaticMesh` _returnvalue))
      (set `self.UseStaticMesh` _asstatic_mesh_2)))
  (`StaticMeshComponent.SetStaticMesh` (`self.StaticMeshComponent`) _output_get))

(event `SetWindForceBlend`
  (params (BlendTime :type "Float (double-precision)") (NewWindDirection :type "Vector Structure"))
  (if (> BlendTime 0.01)
    (set `self.WindDirection` (`KismetMathLibrary.VInterpTo_Constant` (`self.WindDirection`) NewWindDirection (`self.TickWindDirectionInterval`) (/ 1.0 BlendTime)))
    (bind _returnvalue (`MaterialInstanceDynamic.K2_GetVectorParameterValue` (`self.MaterialInstance`) "ForceMin"))
    (`MaterialInstanceDynamic.SetVectorParameterValue` (`self.MaterialInstance`) "ForceMinOld" _returnvalue)
    (bind _returnvalue_2 (`MaterialInstanceDynamic.K2_GetVectorParameterValue` (`self.MaterialInstance`) "ForceMax"))
    (`MaterialInstanceDynamic.SetVectorParameterValue` (`self.MaterialInstance`) "ForceMaxOld" _returnvalue_2)
    (`MaterialInstanceDynamic.SetScalarParameterValue` (`self.MaterialInstance`) "ForceBlend" 0.0)
    (`self.UpdateForce`)
    (`TimelineComponent.SetPlayRate` (`self.WindForceTimeline`) (/ 1.0 (`self.TickWindDirectionInterval`)))
    (bind (_direction _time) (`Timeline|WindForceTimeline` :!via `PlayFromStart`)
      (:`Update`
        (`MaterialInstanceDynamic.SetScalarParameterValue` (`self.MaterialInstance`) "ForceBlend" _time))
      (:`Finished`
        (`self.SetWindForceBlend` (- BlendTime (`self.TickWindDirectionInterval`)) NewWindDirection)))
    (else
      (set `self.WindDirection` NewWindDirection)
      (`self.UpdateForce`)
      (`MaterialInstanceDynamic.SetScalarParameterValue` (`self.MaterialInstance`) "ForceBlend" 1.0))))

(event `SetParticeCountBlend`
  (params (`Target Count` :type Integer :default 5000) (BlendDuration :type "Float (double-precision)") (Animation :type "CurveFloat Object Reference") (RemoveOnEnd :type Boolean))
  (set `self.AnimationDuration` BlendDuration)
  (if (<= (`self.AnimationDuration`) 0.0)
    (set `self.AnimationTime` 1.0)
    (`self.SetParticleCount` `Target Count`)
    (else
      (set `self.AnimationTime` 0.0)
      (set `self.AnimationStartCount` (`self.ParticleCount`))
      (bind _returnvalue (`self.UpdateParticleCount` `Target Count` Animation :!label _label))
      (`self.SetParticleCount` _returnvalue)
      (if (>= (`self.AnimationTime`) 1.0)
        _
        (else
          (`KismetSystemLibrary.Delay` (`self.TickParticleCountInterval`))
          (set `self.AnimationTime` (`KismetMathLibrary.FMin` (+ (`self.AnimationTime`) (/ (`self.TickParticleCountInterval`) (`self.AnimationDuration`))) 1.0))
          (goto _label)))))
  (`self.OnParticlCountBlendFinished` self RemoveOnEnd)
  (if RemoveOnEnd
    (`/Engine/EditorBlueprintResources/StandardMacros.IsValid` self
      (:`Is Valid`
        (`self.K2_DestroyActor` self)))))

(fn `GetPrecipitationAtPoint`
  (params (Location :type "Vector Structure"))
  (returns (Rain :type "Float (double-precision)") (Snow :type "Float (double-precision)") (Wind :type "Float (double-precision)") (Force :type "Vector Structure"))
  (bind _interactwater (`self.InteractWater`))
  (bind (_volumesize_x _volumesize_y _volumesize_z) (`KismetMathLibrary.BreakVector` (`self.VolumeSize`)))
  (bind _interactfreezing (`self.InteractFreezing`))
  (bind _interactwind (`self.InteractWind`))
  (bind (_returnvalue_x _returnvalue_y _returnvalue_z) (`KismetMathLibrary.BreakVector` (`KismetMathLibrary.Vector_GetAbs` (- Location (`SceneComponent.K2_GetComponentLocation` (`self.Box`))))))
  (if (`self.Infinite Extent (Unbound)`)
    _
    (elif (or (or (> _returnvalue_x _volumesize_x) (> _returnvalue_y _volumesize_y)) (> _returnvalue_z _volumesize_z))
      (return 0.0 0.0 0.0 (0.0 0.0 0.0))
      (else
        _)))
  (return (* (* _interactwater _interactwater) (`KismetMathLibrary.Conv_IntToDouble` (`self.ParticleCount`))) (* (* _interactfreezing _interactfreezing) (`KismetMathLibrary.Conv_IntToDouble` (`self.ParticleCount`))) (* (* _interactwind _interactwind) (`KismetMathLibrary.Conv_IntToDouble` (`self.ParticleCount`))) (`KismetMathLibrary.Normal` (+ (`self.GravityForce`) (* (`self.WindDirection`) (`self.WindForce`))))))

(fn `InitStaticMesh`
  (bind _returnvalue (`AddComponent|NODE_AddStaticMeshComponent-0`))
  (set `self.StaticMeshComponent` _returnvalue)
  (`SceneComponent.K2_AttachToComponent` (`self.StaticMeshComponent`) (`self.Box`) "None" "KeepRelative" "KeepRelative" "KeepRelative" true)
  (`PrimitiveComponent.SetCastShadow` (`self.StaticMeshComponent`) false)
  (`PrimitiveComponent.SetCollisionEnabled` (`self.StaticMeshComponent`) "NoCollision")
  (`StaticMeshComponent.SetStaticMesh` (`self.StaticMeshComponent`) (`self.UseStaticMesh`))
  (bind _returnvalue_2 (`PrimitiveComponent.CreateDynamicMaterialInstance` (`self.StaticMeshComponent`) 0 (`self.Material`) "None"))
  (set `self.MaterialInstance` _returnvalue_2)
  (return))

(fn `SetController`
  (params (Controller :type "/Game/InfinityWeather/Weather/Blueprints/BP_InfinityWeatherController Object Reference"))
  (bind _output_get (set `self.Controller` Controller))
  (`/Engine/EditorBlueprintResources/StandardMacros.IsValid` _output_get
    (:`Is Valid`
      (`KismetArrayLibrary.Array_AddUnique` (`/Game/InfinityWeather/Weather/Blueprints/BP_InfinityWeatherController.PrecipitationActors` _output_get) self))))

(fn `SetParticleCount`
  (params (Count :type Integer))
  (bind _output_get (set `self.ParticleCount` Count))
  (`MaterialInstanceDynamic.SetScalarParameterValue` (`self.MaterialInstance`) "ParticleCount" (`KismetMathLibrary.Conv_IntToDouble` _output_get))
  (`AudioComponent.SetFloatParameter` (`self.Audio`) "Fade" (`KismetMathLibrary.FClamp` (* _output_get (/ (`self.SoundIntensityScale`) 65535.0))))
  (`self.UpdateParticleMesh` false))

(fn `SetVolumeSize`
  (params (VolumeSize :type "Vector Structure") (InfiniteExtend :type Boolean))
  (locals (VolumeSizeExt :type "Vector Structure" :default (999999.0 999999.0 999999.0)))
  (set `self.VolumeSize` VolumeSize)
  (set `self.Infinite Extent (Unbound)` InfiniteExtend)
  (`|ExecutionSequence`
    (:`then_0`
      (if (`self.Infinite Extent (Unbound)`)
        (set `local.VolumeSizeExt` (10000000.0 10000000.0 10000000.0))
        (else
          (set `local.VolumeSizeExt` (`self.VolumeSize`)))))
    (:`then_1`
      (`BoxComponent.SetBoxExtent` (`self.Box`) (`local.VolumeSizeExt`) true)
      (bind _outattenuationsettings (`AudioComponent.BP_GetAttenuationSettingsToApply` (`self.Audio`)))
      (bind _structout (setmembers `SoundAttenuationSettings` :`StructRef` _outattenuationsettings :`bSpatialize` (not (`self.Infinite Extent (Unbound)`)) :`AttenuationShapeExtents` (`local.VolumeSizeExt`) :`FalloffDistance` (`self.SoundAttenuationFalloff`)))
      (`AudioComponent.AdjustAttenuation` (`self.Audio`) _structout)
      (`AudioComponent.SetSound` (`self.Audio`) (`AudioComponent.Sound` (`self.Audio`))))
    (:`then_2`
      (`/Engine/EditorBlueprintResources/StandardMacros.IsValid` (`self.MaterialInstance`)
        (:`Is Valid`
          (`MaterialInstanceDynamic.SetVectorParameterValue` (`self.MaterialInstance`) "ClipBoxSize" (`KismetMathLibrary.Conv_VectorToLinearColor` (`local.VolumeSizeExt`))))))))

(fn `SetWindForce`
  (params (BlendDuration :type "Float (double-precision)") (TargetForce :type "Vector Structure"))
  (`self.SetWindForceBlend` BlendDuration TargetForce))

(fn `UpdateForce`
  (locals (LForceScale :type "Vector Structure" :default (0.0 0.0 0.0)) (LForce :type "Vector Structure" :default (0.0 0.0 0.0)))
  (bind _randomforce (`self.RandomForce`))
  (bind _lforce (`local.LForce`))
  (set `local.LForceScale` (/ (`KismetMathLibrary.Conv_DoubleToVector` (`self.PhysicsTickRate`)) (`self.CameraBoxSize`)))
  (set `local.LForce` (+ (`self.GravityForce`) (* (`self.WindDirection`) (`self.WindForce`))))
  (`MaterialInstanceDynamic.SetVectorParameterValue` (`self.MaterialInstance`) "ForceMin" (`KismetMathLibrary.Conv_VectorToLinearColor` (* (`local.LForceScale`) (- _lforce _randomforce))))
  (`MaterialInstanceDynamic.SetVectorParameterValue` (`self.MaterialInstance`) "ForceMax" (`KismetMathLibrary.Conv_VectorToLinearColor` (* (`local.LForceScale`) (+ _lforce _randomforce)))))

(fn `UpdateParticleCount`
  (params (Target :type Integer) (Curve :type "CurveFloat Object Reference (by ref)"))
  (returns (ReturnValue :type Integer))
  (locals (Temp :type "Float (double-precision)" :default 0.0))
  (`/Engine/EditorBlueprintResources/StandardMacros.IsValid` Curve
    (:`Is Valid`
      (set `local.Temp` (`CurveFloat.GetFloatValue` Curve (* (`self.AnimationTime`) (`.MaxTime` (`CurveBase.GetTimeRange` Curve))))))
    (:`Is Not Valid`
      (set `local.Temp` 1.0)))
  (return (`KismetMathLibrary.FTrunc` (`KismetMathLibrary.Lerp` (`KismetMathLibrary.Conv_IntToDouble` (`self.AnimationStartCount`)) (`KismetMathLibrary.Conv_IntToDouble` Target) (* (`KismetMathLibrary.FMin` (`self.AnimationTime`) 1.0) (`local.Temp`))))))

(fn `UpdateParticleMesh`
  (params (Init :type Boolean))
  (locals (ParticleLod :type Integer :default 0) (NewParticleMax :type Integer :default 0) (MeshRef :type "StaticMesh Soft Object Reference"))
  (set `local.ParticleLod` (`KismetMathLibrary.FCeil` (`KismetMathLibrary.Log` (`KismetMathLibrary.Conv_IntToDouble` (`KismetMathLibrary.Max` (`self.ParticleCount`) 1)) 2.0)))
  (set `local.NewParticleMax` (`KismetMathLibrary.FTrunc` (`KismetMathLibrary.MultiplyMultiply_FloatFloat` 2.0 (`KismetMathLibrary.Conv_IntToDouble` (`local.ParticleLod`)))))
  (if (or (!= (`local.NewParticleMax`) (`self.ParticleCountMax`)) (`local.Init`))
    (set `self.ParticleCountMax` (`local.NewParticleMax`))
    (set `local.MeshRef` (`|GetArrayItem` (`self.StaticMeshes`) (`KismetMathLibrary.Clamp` (- (`local.ParticleLod`) 8) 0 (`KismetArrayLibrary.Array_LastIndex` (`self.StaticMeshes`)))))
    (if (`local.Init`)
      (bind _returnvalue (`KismetSystemLibrary.LoadAsset_Blocking` (`local.MeshRef`)))
      (bind _asstatic_mesh (cast `StaticMesh` _returnvalue))
      (set `self.UseStaticMesh` _asstatic_mesh)
      (else
        (`self.AsyncLoadMesh` (`local.MeshRef`))
        (return)))
    (else
      (return))))

(fn `UserConstructionScript`
  (bind _cameraboxdistance (`self.CameraBoxDistance`))
  (bind (_pointsize_x _pointsize_y _pointsize_z) (`KismetMathLibrary.BreakVector` (`self.PointSize`)))
  (`SceneComponent.K2_SetRelativeLocation` (`self.Audio`) (0.0 0.0 0.0) false true)
  (`/Engine/EditorBlueprintResources/StandardMacros.IsValid` (`self.Material`)
    (:`Is Valid`
      (`self.UpdateParticleMesh` true)
      (if (`KismetSystemLibrary.IsValid` (`self.UseStaticMesh`))
        (`self.InitStaticMesh`)
        (`MaterialInstanceDynamic.SetVectorParameterValue` (`self.MaterialInstance`) "PointSize" (make `LinearColor` _pointsize_x _pointsize_y _pointsize_z 1.0))
        (`MaterialInstanceDynamic.SetVectorParameterValue` (`self.MaterialInstance`) "BoxSize" (`KismetMathLibrary.Conv_VectorToLinearColor` (`self.CameraBoxSize`)))
        (`self.SetVolumeSize` (`self.VolumeSize`) (`self.Infinite Extent (Unbound)`))
        (`SceneComponent.K2_SetWorldRotation` :`self` (`self.Box`))
        (`SceneComponent.K2_SetWorldRotation` :`self` (`self.Audio`))
        (`SceneComponent.SetWorldScale3D` (`self.Box`) (1.0 1.0 1.0))
        (`MaterialInstanceDynamic.SetVectorParameterValue` (`self.MaterialInstance`) "CameraOffset" (make `LinearColor` _cameraboxdistance _cameraboxdistance (`self.CameraBoxHeight`) (`self.CameraBoxZOffset`)))
        (`MaterialInstanceDynamic.SetScalarParameterValue` (`self.MaterialInstance`) "Translucency" (`self.Translucency`))
        (`self.UpdateForce`)
        (`self.SetParticleCount` (`self.ParticleCount`))
        (bind _returnvalue (`KismetMaterialLibrary.GetVectorParameterValue` "/Game/InfinityWeather/Weather/Materials/MPC_InfinityWeather.MPC_InfinityWeather" "WindForce"))
        (`self.SetWindForceBlend` 0.0 (`KismetMathLibrary.Conv_LinearColorToVector` _returnvalue))))))