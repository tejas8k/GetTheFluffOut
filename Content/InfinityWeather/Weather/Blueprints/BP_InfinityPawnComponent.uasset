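; Pawn component for the Infinity Weather system that toggles a cold-breath particle effect on its owner.
; BeginPlay caches the weather controller found in the level.
; When enabled, SetOwnerBreath samples temperature at the owner's location and, if below zero, attaches a single emitter to the supplied mesh's socket.
; Disabling deactivates and clears it; temperature is checked only on each call, and warmer readings leave an existing effect running.
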(event `self.ReceiveBeginPlay`
  (bind _returnvalue (`GameplayStatics.GetActorOfClass` "/Game/InfinityWeather/Weather/Blueprints/BP_InfinityWeatherController.BP_InfinityWeatherController_C"))
  (bind _output_get (set `self.Controller` _returnvalue))
  (`/Engine/EditorBlueprintResources/StandardMacros.IsValid` _output_get))

(fn `SetOwnerBreath`
  (params (Enable :type Boolean) (Mesh :type "SkeletalMeshComponent Object Reference"))
  (bind (_breatheffecttransform_location _breatheffecttransform_rotation _breatheffecttransform_scale) (`KismetMathLibrary.BreakTransform` (`self.BreathEffectTransform`)))
  (if Enable
    (`/Engine/EditorBlueprintResources/StandardMacros.IsValid` (`self.Controller`)
      (:`Is Valid`
        (if (and (`self.IsActive`) (`self.UseBreath`))
          (bind _data (`/Game/InfinityWeather/Weather/Blueprints/BP_InfinityWeatherController.GetAtmosphereDataAtLocation` (`self.Controller`) (`Actor.K2_GetActorLocation` (`self.GetOwner`))))
          (if (< (`.Temperature_59_CE6ED57F4C130C870740B288A8FC2A36` (break `/Game/InfinityWeather/Environment/Fog/BS_InfinityAtmosphere` _data)) 0.0)
            (`/Engine/EditorBlueprintResources/StandardMacros.IsValid` (`self.SpawnedBreathEffect`)
              (:`Is Not Valid`
                (bind _returnvalue (`GameplayStatics.SpawnEmitterAttached` (`self.BreathEffect`) (`local.Mesh`) (`self.BreathEffectAttachement`) _breatheffecttransform_location _breatheffecttransform_rotation _breatheffecttransform_scale "KeepRelativeOffset" false "AutoRelease"))
                (set `self.SpawnedBreathEffect` _returnvalue)))))))
    (else
      (`/Engine/EditorBlueprintResources/StandardMacros.IsValid` (`self.SpawnedBreathEffect`)
        (:`Is Valid`
          (`self.Deactivate` (`self.SpawnedBreathEffect`))
          (set `self.SpawnedBreathEffect` null))))))